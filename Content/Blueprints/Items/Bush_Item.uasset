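; Bush_Item is a pickup item that the player collects into the inventory by interacting with it.
; On Interact, it casts the first player character to Cpp_Character and passes a copy of its MainItemStructure fields to AddItemToInventory.
; The actor destroys itself only when that call succeeds, and its construction script just runs the parent's.
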(event `InteractInterface.Interact`
  (bind (_name _thumbnail _itemsize _bisvaliditem) (break `Item_Struct` (`self.Main_Item_Structure`)))
  (bind _ascpp_character (cast `/Game/ThirdPersonBP/Blueprints/Cpp_Character` (`GameplayStatics.GetPlayerCharacter` 0)))
  (bind _returnvalue (`MyCharacter.AddItemToInventory` _ascpp_character (make `Item_Struct` _name _thumbnail _itemsize _bisvaliditem)))
  (if _returnvalue
    (`self.K2_DestroyActor`)))

(fn `UserConstructionScript`
  (`parent.UserConstructionScript`))