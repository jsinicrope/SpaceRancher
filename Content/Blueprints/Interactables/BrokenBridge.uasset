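; Interactable broken bridge that the player repairs with two required inventory items, replacing itself with a RepairedBridge actor at the same transform.
; Interact calls GetRequiredItems up to twice, each removing a named item through Cpp_Character and incrementing CollectedItems, so partial contributions persist between attempts.
; When items are lacking, it shows a RepairBridgeItems widget, which a timer has the character remove shortly after.
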(event `InteractInterface.Interact`
  (bind _success (`self.GetRequiredItems`))
  (if _success
    (if (>= (`self.CollectedItems`) 2)
      (`|SpawnActorFromClass` "/Game/Blueprints/Interactables/RepairedBridge.RepairedBridge_C" (`self.GetTransform`) "Undefined" "OverrideRootScale" null null :!label _label)
      (`self.K2_DestroyActor`)
      (else
        (bind _success_2 (`self.GetRequiredItems`))
        (if _success_2
          (goto _label)
          (else
            (`KismetSystemLibrary.PrintString` "Not enought Items" :!label _label_2)
            (bind _returnvalue (`|CreateWidget` "/Game/Widgets/HUDs/Inventory/RepairBridgeItems.RepairBridgeItems_C" (`GameplayStatics.GetPlayerController` 0)))
            (`UserWidget.AddToViewport` _returnvalue 0)
            (`KismetSystemLibrary.K2_SetTimerDelegate` (delegate `Remove Widget`) 1.5)))))
    (else
      (goto _label_2))))

(event `Remove Widget`
  (bind _ascpp_character (cast `/Game/ThirdPersonBP/Blueprints/Cpp_Character` (`GameplayStatics.GetPlayerCharacter` 0)))
  (set `MyCharacter.WidgetToRemove` (stale `InteractInterface.Interact` _returnvalue) _ascpp_character)
  (`MyCharacter.RemoveWidgetFromViewport` _ascpp_character))

(fn `GetRequiredItems`
  (returns (Success :type Boolean))
  (bind _ascpp_character (cast `/Game/ThirdPersonBP/Blueprints/Cpp_Character` (`GameplayStatics.GetPlayerCharacter` 0)))
  (bind _returnvalue (`MyCharacter.RemoveItemFromInventoryByName` _ascpp_character (`self.RequiredItem`)))
  (if (`.bIsValidItem` (break `Item_Struct` _returnvalue))
    (set `self.CollectedItems` (+ (`self.CollectedItems`) 1))
    (return true)
    (else
      (return false))))

(fn `UserConstructionScript`)