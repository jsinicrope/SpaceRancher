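; BP_DestroyTrigger is a box trigger that destroys a referenced Target actor when a BP_Cpp_Character overlaps it.
; After a configurable delay, it plays a sound at the Target's location and destroys that actor.
; The AbleToDestroy flag is cleared only after destruction, making the trigger single-use; later overlaps just print an "Already Destroyed" debug message.
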(event `self.Box.OnComponentBeginOverlap`
  (params (OverlappedComponent :type "PrimitiveComponent Object Reference") (OtherActor :type "Actor Object Reference") (OtherComp :type "PrimitiveComponent Object Reference") (OtherBodyIndex :type Integer) (bFromSweep :type Boolean) (SweepResult :type "HitResult Structure (by ref)"))
  (bind _rootcomponent (`Actor.RootComponent` (`self.Target`)))
  (cast `/Game/ThirdPersonBP/Blueprints/BP_Cpp_Character` OtherActor)
  (if (`self.AbleToDestroy`)
    (`KismetSystemLibrary.Delay` (`self.DelayTime`))
    (`GameplayStatics.PlaySoundAtLocation` (`self.Sound`) (`SceneComponent.K2_GetComponentLocation` _rootcomponent) (struct) 1.0 1.0 0.0 null null null null)
    (`self.K2_DestroyActor` (`ActorComponent.GetOwner` _rootcomponent))
    (set `self.AbleToDestroy` false)
    (else
      (`KismetSystemLibrary.PrintString` "Already Destroyed" true true (struct :`R` 1.0 :`G` 0.051108 :`A` 1.0)))))

(fn `UserConstructionScript`)